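; BP_Astroneer is the main character Blueprint, which sets up the hero's health, damage and stamina and adds the WPB_Bars widget to the viewport.
; On BeginPlay it loads those stats from the Settings data table, calling the parent's BeginPlay only when the row is found.
; Tick prints health and stamina on screen for debugging, then calls CalculateStamina.
; The 1 key applies test damage to the character itself.
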(event `self.ReceiveBeginPlay`
  ;[1 1 1] Init
  (bind _returnvalue (`|CreateWidget` "/Game/Characters/MainCharacter/UI/WPB_Bars.WPB_Bars_C"))
  (`UserWidget.AddToViewport` _returnvalue 0)
  (bind _returnvalue_2 (`|GetDataTableRow` "/Game/Constants/Settings.Settings" "Settings")
    (:`then`
      (bind _output_get (set `self.Health` (break `/Game/Constants/PresetStruct` _returnvalue_2)))
      (set `self.MaxHealth` _output_get)
      (set `self.Damage` (`.HeroDamage_4_CCF0F34667461B48C6F84D83ED84FBAF` (break `/Game/Constants/PresetStruct` _returnvalue_2)))
      (bind _output_get_2 (set `self.Stamina` (`.HeroMaxStamina_12_20577135584A00B6B73267B4424E8EED` (break `/Game/Constants/PresetStruct` _returnvalue_2))))
      (set `self.MaxStamina` _output_get_2)
      (set `self.StaminaDamage` (`.HeroStaminaTickDamage_14_EFB744A54745E242E8942D96BA1AB962` (break `/Game/Constants/PresetStruct` _returnvalue_2)))
      (`parent.ReceiveBeginPlay`))))

(event `self.ReceiveTick`
  (params (DeltaSeconds :type "Float (single-precision)"))
  ;[1 1 1] Stamina
  (`|ExecutionSequence`
    (:`then_0`
      (`self.ShowHealth`)
      (`self.ShowStamina`))
    (:`then_1`
      (`self.CalculateStamina`))))

(event `Key|One`
  (params (Key :type "Key Structure"))
  (:`Pressed`
    (`GameplayStatics.ApplyDamage` self 10.0)))

(fn `ShowHealth`
  (`KismetSystemLibrary.PrintString` (`KismetStringLibrary.Conv_DoubleToString` (`self.Health`)) true false (struct :`G` 0.66 :`B` 1.0 :`A` 1.0) 0.0))

(fn `ShowStamina`
  (`KismetSystemLibrary.PrintString` (`KismetStringLibrary.Conv_DoubleToString` (`self.Stamina`)) true false (struct :`G` 0.66 :`B` 1.0 :`A` 1.0) 0.0))

(fn `UserConstructionScript`
  (`parent.UserConstructionScript`))