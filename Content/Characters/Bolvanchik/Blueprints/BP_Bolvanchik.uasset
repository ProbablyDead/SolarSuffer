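; Enemy character Bolvanchik, with health, damage and stamina stats and a health bar widget that shows when the player is near.
; On BeginPlay it links itself to the enemy health widget and loads max health, damage, max stamina and stamina damage from the BolvanchikiSettings data table.
; While it is alive, a sphere overlap with BP_Astroneer toggles the widget's visibility, and Tick recalculates stamina.
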(event `self.ReceiveBeginPlay`
  ;[1 1 1] Add health widget
  (bind _asheath_widget_enemy (cast `/Game/Characters/Bolvanchik/UI/HeathWidget_Enemy` (`WidgetComponent.GetUserWidgetObject` (`self.HealthWidget`))))
  (set `/Game/Characters/Bolvanchik/UI/HeathWidget_Enemy.BP_Bolvanchik` self _asheath_widget_enemy)
  (`parent.ReceiveBeginPlay`)
  ;[1 1 1] Applying constants
  (bind _returnvalue (`|GetDataTableRow` "/Game/Constants/VeryEasyLevel/BolvanchikiSettings.BolvanchikiSettings" "Settings")
    (:`then`
      (bind _output_get (set `self.Health` (break `/Game/Constants/ActorsSettings` _returnvalue)))
      (set `self.MaxHealth` _output_get)
      (set `self.Damage` (`.Damage_21_CCF0F34667461B48C6F84D83ED84FBAF` (break `/Game/Constants/ActorsSettings` _returnvalue)))
      (bind _output_get_2 (set `self.Stamina` (`.MaxStamina_22_20577135584A00B6B73267B4424E8EED` (break `/Game/Constants/ActorsSettings` _returnvalue))))
      (set `self.MaxStamina` _output_get_2)
      (set `self.StaminaDamage` (`.StaminaTickDamage_23_EFB744A54745E242E8942D96BA1AB962` (break `/Game/Constants/ActorsSettings` _returnvalue))))))

(event `self.Sphere.OnComponentBeginOverlap`
  (params (OverlappedComponent :type "PrimitiveComponent Object Reference") (OtherActor :type "Actor Object Reference") (OtherComp :type "PrimitiveComponent Object Reference") (OtherBodyIndex :type Integer) (bFromSweep :type Boolean) (SweepResult :type "HitResult Structure (by ref)"))
  ;[1 1 1] Health bar
  (if (not (`self.isDead`))
    (cast `/Game/Characters/MainCharacter/Blueprints/BP_Astroneer` OtherActor)
    (`SceneComponent.SetVisibility` (`self.HealthWidget`) true false)))

(event `self.Sphere.OnComponentEndOverlap`
  (params (OverlappedComponent :type "PrimitiveComponent Object Reference") (OtherActor :type "Actor Object Reference") (OtherComp :type "PrimitiveComponent Object Reference") (OtherBodyIndex :type Integer))
  ;[1 1 1] Health bar
  (if (not (`self.isDead`))
    (cast `/Game/Characters/MainCharacter/Blueprints/BP_Astroneer` OtherActor)
    (`SceneComponent.SetVisibility` (`self.HealthWidget`) false false)))

(event `self.ReceiveTick`
  (params (DeltaSeconds :type "Float (single-precision)"))
  ;[1 1 1] Stamina
  (if (not (`self.isDead`))
    (`self.CalculateStamina`)))

(fn `UserConstructionScript`
  (`parent.UserConstructionScript`))